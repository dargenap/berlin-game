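; First-person player character that spawns an M1911 on BeginPlay, attaches it to the arms' hand socket and maps Enhanced Input actions.
; Movement inputs drive walking, jumping, jog and ADS speeds, plus a timeline-blended crouch, while Tick pitches a pivot with the control rotation.
; DoOnce-gated fire and reload call weapon events and play arm montages, with reload blocking fire until its montage completes.
; Sprint only prints debug text.
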(event Custom|eventUnCrouch
  (bind (_direction _halfheight _walkspeed) (Timeline|tl_Crouch Reverse)
    (:Update
      (Components|Capsule|SetCapsuleHalfHeight (Variables|Collision|GetCapsuleComponent) _halfheight true)
      (Variables|/Script/Engine.CharacterMovementComponent|SetMaxWalkSpeed (Variables|Character|GetCharacterMovement) _walkspeed))))

(event Custom|eventCrouch
  (bind (_direction _halfheight _walkspeed) (Timeline|tl_Crouch Play)
    (:Update
      (Components|Capsule|SetCapsuleHalfHeight (Variables|Collision|GetCapsuleComponent) _halfheight true)
      (Variables|/Script/Engine.CharacterMovementComponent|SetMaxWalkSpeed (Variables|Character|GetCharacterMovement) _walkspeed))))

(event Input|EnhancedActionEvents|EnhancedInputActionIA_Test
  (params (ActionValue :type Boolean) (ElapsedSeconds :type Float%20%28double-precision%29) (TriggeredSeconds :type Float%20%28double-precision%29) (InputAction :type Input%20Action%20Object%20Reference :default "/Game/PlayerCharacter/Logic/Inputs/IA_Test.IA_Test"))
  (Development|PrintString "Hello"))

(event Input|EnhancedActionEvents|EnhancedInputActionIA_Move
  (params (ActionValue :type Vector%202D%20Structure) (ElapsedSeconds :type Float%20%28double-precision%29) (TriggeredSeconds :type Float%20%28double-precision%29) (InputAction :type Input%20Action%20Object%20Reference :default "/Game/PlayerCharacter/Logic/Inputs/IA_Move.IA_Move"))
  (bind (_x _y) (Math|Vector2D|BreakVector2D ActionValue))
  (Pawn|Input|AddMovementInput (* _y (Transformation|GetActorForwardVector)) 1.0 false)
  (Pawn|Input|AddMovementInput (* _x (Transformation|GetActorRightVector)) 1.0 false))

(event Input|EnhancedActionEvents|EnhancedInputActionIA_MouseLook
  (params (ActionValue :type Vector%202D%20Structure) (ElapsedSeconds :type Float%20%28double-precision%29) (TriggeredSeconds :type Float%20%28double-precision%29) (InputAction :type Input%20Action%20Object%20Reference :default "/Game/PlayerCharacter/Logic/Inputs/IA_MouseLook.IA_MouseLook"))
  (bind (_x _y) (Math|Vector2D|BreakVector2D ActionValue))
  (Pawn|Input|AddControllerPitchInput (* _y -1.0))
  (Pawn|Input|AddControllerYawInput _x))

(event Input|EnhancedActionEvents|EnhancedInputActionIA_Jog
  (params (ActionValue :type Boolean) (ElapsedSeconds :type Float%20%28double-precision%29) (TriggeredSeconds :type Float%20%28double-precision%29) (InputAction :type Input%20Action%20Object%20Reference :default "/Game/PlayerCharacter/Logic/Inputs/IA_Jog.IA_Jog"))
  (bind _charactermovement (Variables|Character|GetCharacterMovement))
  (:Triggered
    (Variables|/Script/Engine.CharacterMovementComponent|SetMaxWalkSpeed _charactermovement (Variables|Default|GetmaxJogSpeed)))
  (:Completed
    (Variables|/Script/Engine.CharacterMovementComponent|SetMaxWalkSpeed _charactermovement (Variables|Default|GetdefaultWalkSpeed))))

(event Input|EnhancedActionEvents|EnhancedInputActionIA_Jump
  (params (ActionValue :type Boolean) (ElapsedSeconds :type Float%20%28double-precision%29) (TriggeredSeconds :type Float%20%28double-precision%29) (InputAction :type Input%20Action%20Object%20Reference :default "/Game/PlayerCharacter/Logic/Inputs/IA_Jump.IA_Jump"))
  (Character|Jump))

(event Input|EnhancedActionEvents|EnhancedInputActionIA_Crouch
  (params (ActionValue :type Boolean) (ElapsedSeconds :type Float%20%28double-precision%29) (TriggeredSeconds :type Float%20%28double-precision%29) (InputAction :type Input%20Action%20Object%20Reference :default "/Game/PlayerCharacter/Logic/Inputs/IA_Crouch.IA_Crouch"))
  (:Triggered
    (CallFunction|EventCrouch))
  (:Completed
    (CallFunction|EventUnCrouch)))

(event Input|EnhancedActionEvents|EnhancedInputActionIA_SecondaryFire
  (params (ActionValue :type Boolean) (ElapsedSeconds :type Float%20%28double-precision%29) (TriggeredSeconds :type Float%20%28double-precision%29) (InputAction :type Input%20Action%20Object%20Reference :default "/Game/PlayerCharacter/Logic/Inputs/IA_SecondaryFire.IA_SecondaryFire"))
  (bind _charactermovement (Variables|Character|GetCharacterMovement))
  (:Triggered
    (Variables|Default|SetisAds true)
    (Variables|/Script/Engine.CharacterMovementComponent|SetMaxWalkSpeed _charactermovement (Variables|Default|GetmaxADSSpeed)))
  (:Completed
    (Variables|Default|SetisAds false)
    (Variables|/Script/Engine.CharacterMovementComponent|SetMaxWalkSpeed _charactermovement (Variables|Default|GetdefaultWalkSpeed))))

(event Input|EnhancedActionEvents|EnhancedInputActionIA_PrimaryFire
  (params (ActionValue :type Boolean) (ElapsedSeconds :type Float%20%28double-precision%29) (TriggeredSeconds :type Float%20%28double-precision%29) (InputAction :type Input%20Action%20Object%20Reference :default "/Game/PlayerCharacter/Logic/Inputs/IA_PrimaryFire.IA_PrimaryFire"))
  (bind _currentweapon (Variables|Default|GetCurrentWeapon))
  (:Triggered
    (Utilities|FlowControl|DoOnce false :!label _label
      (:Completed
        (Default|EventPrimaryFire _currentweapon)
        (if (Variables|/Game/Items/Weapons/Guns/BP_WEP_m1911.BP_WEP_m1911_C|GetcanFire _currentweapon)
          (Animation|Montage|PlayMontage (Variables|Default|GetCharacterArms) "/Game/Characters/Mannequins/Anims/new/m1911/AM_m1911_fire_ads.AM_m1911_fire_ads")))))
  (:Completed
    (goto _label Reset)))

(event Input|EnhancedActionEvents|EnhancedInputActionIA_Sprint
  (params (ActionValue :type Boolean) (ElapsedSeconds :type Float%20%28double-precision%29) (TriggeredSeconds :type Float%20%28double-precision%29) (InputAction :type Input%20Action%20Object%20Reference :default "/Game/PlayerCharacter/Logic/Inputs/IA_Sprint.IA_Sprint"))
  (Development|PrintString "sprint"))

(event Input|EnhancedActionEvents|EnhancedInputActionIA_Reload
  (params (ActionValue :type Boolean) (ElapsedSeconds :type Float%20%28double-precision%29) (TriggeredSeconds :type Float%20%28double-precision%29) (InputAction :type Input%20Action%20Object%20Reference :default "/Game/PlayerCharacter/Logic/Inputs/IA_Reload.IA_Reload"))
  (bind _currentweapon (Variables|Default|GetCurrentWeapon))
  (:Triggered
    (Utilities|FlowControl|DoOnce false :!label _label
      (:Completed
        (Variables|/Game/Items/Weapons/Guns/BP_WEP_m1911.BP_WEP_m1911_C|SetcanFire _currentweapon false)
        (Animation|Montage|PlayMontage (Variables|Default|GetCharacterArms) "/Game/Characters/Mannequins/Anims/new/m1911/AM_m1911_reload.AM_m1911_reload"
          (:OnCompleted
            (Default|EventReload _currentweapon)
            (Variables|/Game/Items/Weapons/Guns/BP_WEP_m1911.BP_WEP_m1911_C|SetcanFire _currentweapon true)
            (goto _label Reset)))))))

(event EventBeginPlay
  (Input|AddMappingContext (PlayerController|LocalPlayerSubsystems|GetEnhancedInputLocalPlayerSubsystem (Game|GetPlayerController 0)) "/Game/PlayerCharacter/Logic/IMC_FPS_Default.IMC_FPS_Default" 0 "(bIgnoreAllPressedKeysUntilRelease=True,bForceImmediately=False,bNotifyUserSettings=False)")
  (bind _returnvalue (Game|SpawnActorfromClass "/Game/Items/Weapons/Guns/BP_WEP_m1911.BP_WEP_m1911_C" (Math|Transform|MakeTransform "0, 0, 0" "0, 0, 0" "1.000000,1.000000,1.000000") "Undefined" "MultiplyWithRoot" 0 0))
  (bind _output_get (Variables|Default|SetCurrentWeapon _returnvalue))
  (Transformation|AttachComponentToComponent _output_get (Variables|Default|GetCharacterArms) "HandGrip_R" "KeepRelative" "KeepRelative" "KeepRelative" true))

(event Collision|EventActorBeginOverlap
  (params (OtherActor :type Actor%20Object%20Reference)))

(event EventTick
  (params (DeltaSeconds :type Float%20%28single-precision%29))
  (Transformation|SetRelativeRotation (Variables|Default|GetPivot) (Math|Rotator|MakeRotator 0.0 (.Pitch (Math|Rotator|BreakRotator (Pawn|GetControlRotation :!class /Script/Engine.Pawn))) 0.0) false false))

(fn ConstructionScript)