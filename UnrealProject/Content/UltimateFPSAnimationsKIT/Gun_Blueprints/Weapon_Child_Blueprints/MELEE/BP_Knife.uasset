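; Melee knife weapon, a child weapon Blueprint with primary and secondary swings plus draw and undraw montages on the player's arms.
; Each swing plays its montage, runs a short camera line trace with random spread, then holds a shared cooldown flag, longer for the secondary.
; The trace result places a knife decal, with separate rotation math for upward-facing floors and other surfaces.
; No damage is applied in these graphs.
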(event Custom|Draw
  (Utilities|DrawMacro))

(event Custom|Undraw
  (bind _returnvalue (Utilities|UndrawMacro))
  (Variables|Default|SetUndrawTime _returnvalue))

(event EventSecondartAttack
  (if (not (Variables|Default|GetKnifeSwingDelay))
    (Variables|Default|SetKnifeSwingDelay true)
    (Utilities|FlowControl|Sequence
      (:then_0
        (Animation|Montage|PlayMontage (Variables|/Game/UltimateFPSAnimationsKIT/Demo/PlayerMannequin/BP_PlayerCharacter.BP_PlayerCharacter_C|GetArms (.AsBP%20Player%20Character (Utilities|Casting|CastToBP_PlayerCharacter (Game|GetPlayerCharacter 0)))) "/Game/UltimateFPSAnimationsKIT/Animations/Arms_Montages/knife_arms_Swing_2_Montage.knife_arms_Swing_2_Montage"))
      (:then_1
        (bind (_impactpoint _impactnormal) (CallFunction|LineTrace))
        (CallFunction|SpawnBulletProjectile _impactnormal _impactpoint))
      (:then_2
        (Utilities|FlowControl|RetriggerableDelay 1.0)
        (Variables|Default|SetKnifeSwingDelay false)))))

(event EventFire
  (if (not (Variables|Default|GetKnifeSwingDelay))
    (Variables|Default|SetKnifeSwingDelay true)
    (Utilities|FlowControl|Sequence
      (:then_0
        (Animation|Montage|PlayMontage (Variables|/Game/UltimateFPSAnimationsKIT/Demo/PlayerMannequin/BP_PlayerCharacter.BP_PlayerCharacter_C|GetArms (.AsBP%20Player%20Character (Utilities|Casting|CastToBP_PlayerCharacter (Game|GetPlayerCharacter 0)))) "/Game/UltimateFPSAnimationsKIT/Animations/Arms_Montages/knife_arms_Swing_1_Montage.knife_arms_Swing_1_Montage"))
      (:then_1
        (bind (_impactpoint _impactnormal) (CallFunction|LineTrace))
        (CallFunction|SpawnBulletProjectile _impactnormal _impactpoint))
      (:then_2
        (Utilities|FlowControl|RetriggerableDelay 0.5)
        (Variables|Default|SetKnifeSwingDelay false)))))

(fn ConstructionScript
  (|CallParentFunction)
  (Variables|Default|SetName "NewEnumerator0")
  (Variables|Default|SetVariableMode true))

(fn LineTrace
  (bind _returnvalue (Game|GetPlayerCharacter 0))
  (bind _bulletspread (Variables|Default|GetBulletSpread))
  (bind _asbp_player_character (Utilities|Casting|CastToBP_PlayerCharacter _returnvalue))
  (bind _returnvalue_2 (* _bulletspread -1.0))
  (bind _playercamera (Variables|/Game/UltimateFPSAnimationsKIT/Demo/PlayerMannequin/BP_PlayerCharacter.BP_PlayerCharacter_C|GetPlayerCamera _asbp_player_character))
  (bind _returnvalue_3 (Transformation|GetWorldLocation _playercamera))
  (bind (_outhit _returnvalue_4) (Collision|LineTraceByChannel _returnvalue_3 (+ (+ (* (Math|Vector|GetForwardVector _playercamera) 175.0) _returnvalue_3) (Math|Vector|MakeVector (Math|Random|RandomFloatinRange _returnvalue_2 _bulletspread) (Math|Random|RandomFloatinRange _returnvalue_2 _bulletspread) (Math|Random|RandomFloatinRange _returnvalue_2 _bulletspread))) "TraceTypeQuery1" false 0 "None")) ; CameraLineTrace
  (if _returnvalue_4
    (return (.ImpactPoint (Collision|BreakHitResult _outhit)) (.ImpactNormal (Collision|BreakHitResult _outhit)))))

(fn SpawnBulletProjectile
  (params (ImpactNormal :type Vector) (ImpactPoint :type Vector))
  (bind _returnvalue (Math|Conversions|RotationFromXVector ImpactNormal))
  (bind _returnvalue_2 (Game|GetPlayerCharacter 0))
  (bind _asbp_player_character (Utilities|Casting|CastToBP_PlayerCharacter _returnvalue_2))
  (bind _playercamera (Variables|/Game/UltimateFPSAnimationsKIT/Demo/PlayerMannequin/BP_PlayerCharacter.BP_PlayerCharacter_C|GetPlayerCamera _asbp_player_character))
  (if (Utilities|Operators|EqualEqual ImpactNormal "0,0,1.000000" 0.0001)
    (Game|SpawnActorfromClass "/Game/UltimateFPSAnimationsKIT/Gun_Blueprints/BP_KnifeDecal.BP_KnifeDecal_C" (Math|Transform|MakeTransform ImpactPoint (Math|Rotator|MakeRotator -9e+01 9e+01 (.yaw (Math|Conversions|RotationFromXVector (Math|Vector|GetForwardVector _playercamera)))) "0.100000,0.060000,0.060000") "Undefined" "OverrideRootScale" 0 0)
    (else
      (Game|SpawnActorfromClass "/Game/UltimateFPSAnimationsKIT/Gun_Blueprints/BP_KnifeDecal.BP_KnifeDecal_C" (Math|Transform|MakeTransform ImpactPoint (Math|Rotator|MakeRotator (+ (.roll (Transformation|GetWorldRotation _playercamera)) 9e+01) (.pitch _returnvalue) (+ (.yaw _returnvalue) 1.8e+02)) "0.100000,0.060000,0.060000") "Undefined" "OverrideRootScale" 0 0)))
  (return))