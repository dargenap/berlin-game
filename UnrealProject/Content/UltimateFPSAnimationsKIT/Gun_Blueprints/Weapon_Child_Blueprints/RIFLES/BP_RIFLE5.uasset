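; RIFLE5 weapon child Blueprint for the FPS kit, handling single or gated automatic fire, reloading and equip/draw animations on BP_PlayerCharacter.
; Each shot traces from the camera with random spread, spawns bullet, decal and shell, and plays montages and muzzle flash.
; An aim-down-sights recoil timeline kicks the view, then reverses with compensation scaled by pitch drift.
; Reloads vary by aim and empty state; undrawing saves weapon stats to the character.
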(event Custom|Draw
  ;[1 1 1] Draw
  (Utilities|DrawMacro))

(event Custom|Undraw
  ;[1 1 1] Undraw
  (bind _returnvalue (Utilities|UndrawMacro)
    (:Completed
      (Variables|Default|SetUndrawTime _returnvalue))))

(event EventReload
  (bind _returnvalue (Game|GetPlayerCharacter 0))
  (bind _returnvalue_2 (Game|GetPlayerCharacter 0))
  (bind _primaryweapon (Variables|Default|GetPrimaryWeapon))
  (bind _asbp_player_character (Utilities|Casting|CastToBP_PlayerCharacter _returnvalue_2))
  (bind _asbp_player_character_2 (Utilities|Casting|CastToBP_PlayerCharacter _returnvalue))
  (bind _aimdownsight (Variables|/Game/UltimateFPSAnimationsKIT/Demo/PlayerMannequin/BP_PlayerCharacter.BP_PlayerCharacter_C|GetAimDownSight _asbp_player_character_2))
  (bind _arms (Variables|/Game/UltimateFPSAnimationsKIT/Demo/PlayerMannequin/BP_PlayerCharacter.BP_PlayerCharacter_C|GetArms _asbp_player_character_2))
  ;[1 1 1] Reload
  (if (< (Variables|Default|GetAmmoCount) (Variables|Default|GetMaxAmmo))
    (if (< (Variables|Default|GetAmmoCount) 1)
      (if _aimdownsight
        (Utilities|FlowControl|DoOnce false :!label _label
          (:Completed
            (Variables|/Game/UltimateFPSAnimationsKIT/Demo/PlayerMannequin/BP_PlayerCharacter.BP_PlayerCharacter_C|SetIsReloading _asbp_player_character_2 true)
            (Animation|Montage|MontagePlay (Components|SkeletalMesh|GetAnimInstance _arms) "/Game/UltimateFPSAnimationsKIT/Animations/Arms_Montages/RIFLE5_arms_reload_empty__ads_Montage.RIFLE5_arms_reload_empty__ads_Montage" 1.0 "MontageLength" 0.0 true)
            (Utilities|FlowControl|Sequence
              (:then_0
                (Components|Animation|PlayAnimation (Variables|Default|GetPrimaryWeapon) "/Game/UltimateFPSAnimationsKIT/Animations/Gun/RIFLE5_gun_reload_empty.RIFLE5_gun_reload_empty" false)
                (Utilities|FlowControl|Delay (Variables|Default|GetReloadTime))
                (Variables|Default|SetAmmoCount (Variables|Default|GetMaxAmmo))
                (Variables|/Game/UltimateFPSAnimationsKIT/Demo/PlayerMannequin/BP_PlayerCharacter.BP_PlayerCharacter_C|SetIsReloading _asbp_player_character false)
                (goto _label Reset))
              (:then_1
                _))))
        (else
          (Utilities|FlowControl|DoOnce false :!label _label_2
            (:Completed
              (Variables|/Game/UltimateFPSAnimationsKIT/Demo/PlayerMannequin/BP_PlayerCharacter.BP_PlayerCharacter_C|SetIsReloading _asbp_player_character_2 true)
              (CallFunction|HideAmmo)
              (Animation|Montage|MontagePlay (Components|SkeletalMesh|GetAnimInstance _arms) "/Game/UltimateFPSAnimationsKIT/Animations/Arms_Montages/RIFLE5_arms_reload_empty__Montage.RIFLE5_arms_reload_empty__Montage" 1.0 "MontageLength" 0.0 true)
              (Utilities|FlowControl|Sequence
                (:then_0
                  (Components|Animation|PlayAnimation (Variables|Default|GetPrimaryWeapon) "/Game/UltimateFPSAnimationsKIT/Animations/Gun/RIFLE5_gun_reload_empty.RIFLE5_gun_reload_empty" false)
                  (Utilities|FlowControl|Delay (Variables|Default|GetReloadTime))
                  (Variables|Default|SetAmmoCount (Variables|Default|GetMaxAmmo))
                  (Variables|/Game/UltimateFPSAnimationsKIT/Demo/PlayerMannequin/BP_PlayerCharacter.BP_PlayerCharacter_C|SetIsReloading _asbp_player_character false)
                  (goto _label_2 Reset))
                (:then_1
                  _))))))
      ;;[1 1 1] Mag Spawn
      (Utilities|FlowControl|Sequence
        (:then_0
          (Utilities|FlowControl|Delay 0.8)
          (Game|SpawnActorfromClass "/Game/UltimateFPSAnimationsKIT/Gun_Blueprints/MagDrops/BP_Mag_Rifle5.BP_Mag_Rifle5_C" (Transformation|GetSocketTransform (Variables|Default|GetPrimaryWeapon) "magSocket" "RTS_World") "Undefined" "OverrideRootScale" 0 0))
        (:then_1
          ;;[1 1 1] Hiding Mag
          (Utilities|FlowControl|Delay 0.2)
          (Components|SkinnedMesh|HideBonebyName _primaryweapon "mag" "PBO_None")
          (Components|SkinnedMesh|HideBonebyName _primaryweapon "bullet" "PBO_None")
          (Components|SkinnedMesh|HideBonebyName _primaryweapon "bullets" "PBO_None")
          (Utilities|FlowControl|Delay 0.8)
          (Components|SkinnedMesh|UnHideBonebyName _primaryweapon "mag")
          (Components|SkinnedMesh|UnHideBonebyName _primaryweapon "bullet")
          (Components|SkinnedMesh|UnHideBonebyName _primaryweapon "bullets")))
      (elif _aimdownsight
        (Utilities|FlowControl|DoOnce false :!label _label_3
          (:Completed
            (Variables|/Game/UltimateFPSAnimationsKIT/Demo/PlayerMannequin/BP_PlayerCharacter.BP_PlayerCharacter_C|SetIsReloading _asbp_player_character_2 true)
            (Animation|Montage|MontagePlay (Components|SkeletalMesh|GetAnimInstance _arms) "/Game/UltimateFPSAnimationsKIT/Animations/Arms_Montages/RIFLE5_arms_reload_ads_Montage.RIFLE5_arms_reload_ads_Montage" 1.0 "MontageLength" 0.0 true)
            (Components|Animation|PlayAnimation (Variables|Default|GetPrimaryWeapon) "/Game/UltimateFPSAnimationsKIT/Animations/Gun/RIFLE5_gun_reload.RIFLE5_gun_reload" false)
            (Utilities|FlowControl|Delay (Variables|Default|GetReloadTime))
            (Variables|Default|SetAmmoCount (Variables|Default|GetMaxAmmo))
            (Variables|/Game/UltimateFPSAnimationsKIT/Demo/PlayerMannequin/BP_PlayerCharacter.BP_PlayerCharacter_C|SetIsReloading _asbp_player_character false)
            (goto _label_3 Reset)))
        (else
          (Utilities|FlowControl|DoOnce false :!label _label_4
            (:Completed
              (Variables|/Game/UltimateFPSAnimationsKIT/Demo/PlayerMannequin/BP_PlayerCharacter.BP_PlayerCharacter_C|SetIsReloading _asbp_player_character_2 true)
              (Animation|Montage|MontagePlay (Components|SkeletalMesh|GetAnimInstance _arms) "/Game/UltimateFPSAnimationsKIT/Animations/Arms_Montages/RIFLE5_arms_reload_Montage.RIFLE5_arms_reload_Montage" 1.0 "MontageLength" 0.0 true)
              (Components|Animation|PlayAnimation (Variables|Default|GetPrimaryWeapon) "/Game/UltimateFPSAnimationsKIT/Animations/Gun/RIFLE5_gun_reload.RIFLE5_gun_reload" false)
              (Utilities|FlowControl|Delay (Variables|Default|GetReloadTime))
              (Variables|Default|SetAmmoCount (Variables|Default|GetMaxAmmo))
              (Variables|/Game/UltimateFPSAnimationsKIT/Demo/PlayerMannequin/BP_PlayerCharacter.BP_PlayerCharacter_C|SetIsReloading _asbp_player_character false)
              (goto _label_4 Reset))))))))

(event EventHideMuzzleFlash
  ;[1 1 1] Hide/UnhideMuzzleflash
  (Rendering|Material|SetMaterial (Variables|Default|GetMuzzelFlashPlane) 0 "/Game/UltimateFPSAnimationsKIT/GunModels/Materials/M_Transparent.M_Transparent")
  (Rendering|SetVisibility (Variables|Default|GetPointLight) false false))

(event EventFire
  (bind _returnvalue (Game|GetPlayerCharacter 0))
  (bind _returnvalue_2 (Game|GetPlayerCharacter 0))
  (bind _returnvalue_3 (Game|GetPlayerController 0))
  (bind _returnvalue_4 (Game|GetPlayerCharacter 0))
  (bind _recoilpattern (Variables|Default|GetRecoilPattern))
  (bind _maxrecoilthreshold (Variables|Default|GetMaxRecoilThreshold))
  (bind _asbp_player_character (Utilities|Casting|CastToBP_PlayerCharacter _returnvalue))
  (bind _asbp_player_character_2 (Utilities|Casting|CastToBP_PlayerCharacter _returnvalue_2))
  (bind _asbp_player_character_3 (Utilities|Casting|CastToBP_PlayerCharacter _returnvalue_4))
  (bind _arms (Variables|/Game/UltimateFPSAnimationsKIT/Demo/PlayerMannequin/BP_PlayerCharacter.BP_PlayerCharacter_C|GetArms _asbp_player_character_3))
  (bind _aimdownsight (Variables|/Game/UltimateFPSAnimationsKIT/Demo/PlayerMannequin/BP_PlayerCharacter.BP_PlayerCharacter_C|GetAimDownSight _asbp_player_character_2))
  ;[1 1 1] Fire
  (if (Variables|Default|GetWeaponMode)
    (Utilities|FlowControl|Sequence
      (:then_0
        (if (> (Variables|Default|GetAmmoCount) 0) :!label _label
          ;[1 1 1] Recoil
          (Utilities|FlowControl|Sequence
            (:then_0
              (Utilities|FlowControl|Sequence
                (:then_0
                  (Utilities|FlowControl|DoOnce false :!label _label_2
                    (:Completed
                      (Variables|Default|SetOGControllerRotation (Pawn|GetControlRotation (Game|GetPlayerController 0) :!class /Script/Engine.Controller)))))
                (:then_1
                  (Components|Timeline|SetPlayRate _recoilpattern 1.0)
                  (bind (_direction _pitch _yaw) (Timeline|RecoilPattern Play)
                    (:Update
                      (if _aimdownsight
                        (if (> (Variables|Default|GetAmmoCount) 0)
                          (switch Utilities|FlowControl|Switch|SwitchonETimelineDirection _direction
                            (:Forward
                              (Class|PlayerController|AddPitchInput _returnvalue_3 _pitch)
                              (Class|PlayerController|AddYawInput _returnvalue_3 _yaw))
                            (:Backward
                              (Utilities|FlowControl|Sequence
                                (:then_0
                                  (Utilities|FlowControl|DoOnce false :!label _label_3
                                    (:Completed
                                      (Variables|Default|SetPostRecoilRotation (Pawn|GetControlRotation (Game|GetPlayerController 0) :!class /Script/Engine.Controller)))))
                                (:then_1
                                  (Class|PlayerController|AddPitchInput _returnvalue_3 (* _pitch -8.0 (select (> (Math|Float|Absolute(Float) (.Pitch (Math|Rotator|BreakRotator (Math|Rotator|Delta(Rotator) (Variables|Default|GetOGControllerRotation) (Variables|Default|GetPostRecoilRotation))))) _maxrecoilthreshold) (Math|Float|MapRangeClamped (Math|Float|Absolute(Float) (.Pitch (Math|Rotator|BreakRotator (Math|Rotator|Delta(Rotator) (Variables|Default|GetOGControllerRotation) (Variables|Default|GetPostRecoilRotation))))) _maxrecoilthreshold 3e+01 1.0 0.0) (Math|Float|MapRangeClamped (Math|Float|Absolute(Float) (.Pitch (Math|Rotator|BreakRotator (Math|Rotator|Delta(Rotator) (Variables|Default|GetOGControllerRotation) (Variables|Default|GetPostRecoilRotation))))) 0.0 _maxrecoilthreshold 0.0 1.0))))
                                  (Class|PlayerController|AddYawInput _returnvalue_3 (* _yaw -1.0 (select (> (Math|Float|Absolute(Float) (.Pitch (Math|Rotator|BreakRotator (Math|Rotator|Delta(Rotator) (Variables|Default|GetOGControllerRotation) (Variables|Default|GetPostRecoilRotation))))) _maxrecoilthreshold) (Math|Float|MapRangeClamped (Math|Float|Absolute(Float) (.Pitch (Math|Rotator|BreakRotator (Math|Rotator|Delta(Rotator) (Variables|Default|GetOGControllerRotation) (Variables|Default|GetPostRecoilRotation))))) _maxrecoilthreshold 3e+01 1.0 0.0) (Math|Float|MapRangeClamped (Math|Float|Absolute(Float) (.Pitch (Math|Rotator|BreakRotator (Math|Rotator|Delta(Rotator) (Variables|Default|GetOGControllerRotation) (Variables|Default|GetPostRecoilRotation))))) 0.0 _maxrecoilthreshold 0.0 1.0)))))))))))
                    (:Finished
                      (if _aimdownsight
                        (switch Utilities|FlowControl|Switch|SwitchonETimelineDirection _direction
                          (:Backward
                            (Utilities|FlowControl|Sequence
                              (:then_0
                                (goto _label_2 Reset))
                              (:then_1
                                (goto _label_3 Reset)))))))))))
            (:then_1
              (CallFunction|AmmoCheck)
              (bind (_muzzlelocation _impactpoint _projectilerotation) (CallFunction|LineTrace))
              (CallFunction|SpawnBulletProjectile _muzzlelocation _impactpoint _impactpoint _projectilerotation)
              (if (Variables|/Game/UltimateFPSAnimationsKIT/Demo/PlayerMannequin/BP_PlayerCharacter.BP_PlayerCharacter_C|GetAimDownSight _asbp_player_character_3)
                (Animation|Montage|PlayMontage _arms "/Game/UltimateFPSAnimationsKIT/Animations/Arms_Montages/RIFLE5_arms_fire_ads_Montage.RIFLE5_arms_fire_ads_Montage"
                  (:then
                    _))
                (else
                  (Animation|Montage|PlayMontage _arms "/Game/UltimateFPSAnimationsKIT/Animations/Arms_Montages/RIFLE5_arms_fire_Montage.RIFLE5_arms_fire_Montage"
                    (:then
                      _))))
              (Utilities|MuzzleFlash)
              (Utilities|EjectShell)
              (if (not (Variables|/Game/UltimateFPSAnimationsKIT/Demo/PlayerMannequin/BP_PlayerCharacter.BP_PlayerCharacter_C|GetAimDownSight _asbp_player_character))
                (Default|IncreaseSpread _asbp_player_character 0.06))))
          (else
            (Audio|PlaySound2D "/Game/UltimateFPSAnimationsKIT/SoundFX/dryfire.dryfire" 1.0 1.0 0.0 0 0))))
      (:then_1
        (Utilities|FlowControl|Delay 0.1)
        (Components|Timeline|SetPlayRate _recoilpattern 8.0)
        (Timeline|RecoilPattern Reverse)))
    (else
      (Utilities|FlowControl|Sequence
        (:then_0
          (goto _label_4 Open))
        (:then_1
          (Utilities|FlowControl|Gate true :!label _label_4
            (:Exit
              (Utilities|FlowControl|Sequence
                (:then_0
                  (goto _label))
                (:then_1
                  (Utilities|FlowControl|RetriggerableDelay 0.12)
                  (goto _label_4))))))))))

(event EventUnhideMuzzleFlash
  ;[1 1 1] Hide/UnhideMuzzleflash
  (Rendering|Material|SetMaterial (Variables|Default|GetMuzzelFlashPlane) 0 "/Game/UltimateFPSAnimationsKIT/TexturesAndMats/M_MuzzleFlash.M_MuzzleFlash")
  (Rendering|SetVisibility (Variables|Default|GetPointLight) true false))

(event EventEquipe
  (bind _returnvalue (Game|GetPlayerCharacter 0))
  (bind _asbp_player_character (Utilities|Casting|CastToBP_PlayerCharacter _returnvalue))
  ;[1 1 1] Equipe
  (Animation|Montage|MontagePlay (Components|SkeletalMesh|GetAnimInstance (Variables|/Game/UltimateFPSAnimationsKIT/Demo/PlayerMannequin/BP_PlayerCharacter.BP_PlayerCharacter_C|GetArms _asbp_player_character)) "/Game/UltimateFPSAnimationsKIT/Animations/Arms_Montages/RIFLE5_arms_equipe_Montage.RIFLE5_arms_equipe_Montage" 1.0 "MontageLength" 0.0 true)
  (Components|Animation|PlayAnimation (Variables|Default|GetPrimaryWeapon) "/Game/UltimateFPSAnimationsKIT/Animations/Gun/RIFLE5_gun_equipe.RIFLE5_gun_equipe" false)
  (Variables|/Game/UltimateFPSAnimationsKIT/Demo/PlayerMannequin/BP_PlayerCharacter.BP_PlayerCharacter_C|SetKnifeActive _asbp_player_character false))

(event EventStopFiring
  (bind _returnvalue (Game|GetPlayerCharacter 0))
  (bind _returnvalue_2 (Game|GetPlayerCharacter 0))
  (bind _returnvalue_3 (Game|GetPlayerController 0))
  (bind _returnvalue_4 (Game|GetPlayerCharacter 0))
  (bind _recoilpattern (Variables|Default|GetRecoilPattern))
  (bind _maxrecoilthreshold (Variables|Default|GetMaxRecoilThreshold))
  (bind _asbp_player_character (Utilities|Casting|CastToBP_PlayerCharacter _returnvalue))
  (bind _asbp_player_character_2 (Utilities|Casting|CastToBP_PlayerCharacter _returnvalue_2))
  (bind _asbp_player_character_3 (Utilities|Casting|CastToBP_PlayerCharacter _returnvalue_4))
  (bind _arms (Variables|/Game/UltimateFPSAnimationsKIT/Demo/PlayerMannequin/BP_PlayerCharacter.BP_PlayerCharacter_C|GetArms _asbp_player_character_3))
  (bind _aimdownsight (Variables|/Game/UltimateFPSAnimationsKIT/Demo/PlayerMannequin/BP_PlayerCharacter.BP_PlayerCharacter_C|GetAimDownSight _asbp_player_character_2))
  ;[1 1 1] Fire
  (Utilities|FlowControl|Sequence
    (:then_0
      (Utilities|FlowControl|Gate true) ; enters at Close
    )
    (:then_1
      ;[1 1 1] Recoil
      (Components|Timeline|SetPlayRate _recoilpattern 8.0)
      (bind (_direction _pitch _yaw) (Timeline|RecoilPattern Reverse)
        (:Update
          (if _aimdownsight
            (if (> (Variables|Default|GetAmmoCount) 0)
              (switch Utilities|FlowControl|Switch|SwitchonETimelineDirection _direction
                (:Forward
                  (Class|PlayerController|AddPitchInput _returnvalue_3 _pitch)
                  (Class|PlayerController|AddYawInput _returnvalue_3 _yaw))
                (:Backward
                  (Utilities|FlowControl|Sequence
                    (:then_0
                      (Utilities|FlowControl|DoOnce false :!label _label
                        (:Completed
                          (Variables|Default|SetPostRecoilRotation (Pawn|GetControlRotation (Game|GetPlayerController 0) :!class /Script/Engine.Controller)))))
                    (:then_1
                      (Class|PlayerController|AddPitchInput _returnvalue_3 (* _pitch -8.0 (select (> (Math|Float|Absolute(Float) (.Pitch (Math|Rotator|BreakRotator (Math|Rotator|Delta(Rotator) (Variables|Default|GetOGControllerRotation) (Variables|Default|GetPostRecoilRotation))))) _maxrecoilthreshold) (Math|Float|MapRangeClamped (Math|Float|Absolute(Float) (.Pitch (Math|Rotator|BreakRotator (Math|Rotator|Delta(Rotator) (Variables|Default|GetOGControllerRotation) (Variables|Default|GetPostRecoilRotation))))) _maxrecoilthreshold 3e+01 1.0 0.0) (Math|Float|MapRangeClamped (Math|Float|Absolute(Float) (.Pitch (Math|Rotator|BreakRotator (Math|Rotator|Delta(Rotator) (Variables|Default|GetOGControllerRotation) (Variables|Default|GetPostRecoilRotation))))) 0.0 _maxrecoilthreshold 0.0 1.0))))
                      (Class|PlayerController|AddYawInput _returnvalue_3 (* _yaw -1.0 (select (> (Math|Float|Absolute(Float) (.Pitch (Math|Rotator|BreakRotator (Math|Rotator|Delta(Rotator) (Variables|Default|GetOGControllerRotation) (Variables|Default|GetPostRecoilRotation))))) _maxrecoilthreshold) (Math|Float|MapRangeClamped (Math|Float|Absolute(Float) (.Pitch (Math|Rotator|BreakRotator (Math|Rotator|Delta(Rotator) (Variables|Default|GetOGControllerRotation) (Variables|Default|GetPostRecoilRotation))))) _maxrecoilthreshold 3e+01 1.0 0.0) (Math|Float|MapRangeClamped (Math|Float|Absolute(Float) (.Pitch (Math|Rotator|BreakRotator (Math|Rotator|Delta(Rotator) (Variables|Default|GetOGControllerRotation) (Variables|Default|GetPostRecoilRotation))))) 0.0 _maxrecoilthreshold 0.0 1.0)))))))))))
        (:Finished
          (if _aimdownsight
            (switch Utilities|FlowControl|Switch|SwitchonETimelineDirection _direction
              (:Backward
                (Utilities|FlowControl|Sequence
                  (:then_0
                    (Utilities|FlowControl|DoOnce false) ; enters at Reset
                  )
                  (:then_1
                    (goto _label Reset)))))))))))

(fn ConstructionScript
  (|CallParentFunction)
  (Variables|Default|SetMaxAmmo 30)
  (Variables|Default|SetAmmoCount 30)
  (Variables|Default|SetReloadTime 2.0)
  (Variables|Default|SetBulletSpread 5e+02)
  (Variables|Default|SetName "NewEnumerator20")
  (Variables|Default|SetVariableMode true))

(fn AmmoCheck
  (Math|Integer|DecrementInt (Variables|Default|GetAmmoCount)
    (:%20%20
      (if (not (Variables|/Game/UltimateFPSAnimationsKIT/Demo/PlayerMannequin/BP_PlayerCharacter.BP_PlayerCharacter_C|GetIsReloading (.AsBP%20Player%20Character (Utilities|Casting|CastToBP_PlayerCharacter (Game|GetPlayerCharacter 0)))))
        (Components|Animation|PlayAnimation (Variables|Default|GetPrimaryWeapon) "/Game/UltimateFPSAnimationsKIT/Animations/Gun/RIFLE5_gun_fire.RIFLE5_gun_fire" false)))))

(fn LineTrace
  (bind _returnvalue (Game|GetPlayerCharacter 0))
  (bind _returnvalue_2 (Game|GetPlayerCharacter 0))
  (bind _bulletspread (Variables|Default|GetBulletSpread))
  (bind _muzzle (Variables|Default|GetMuzzle))
  (bind _returnvalue_3 (Transformation|GetWorldLocation _muzzle))
  (bind _asbp_player_character (Utilities|Casting|CastToBP_PlayerCharacter _returnvalue))
  (bind _asbp_player_character_2 (Utilities|Casting|CastToBP_PlayerCharacter _returnvalue_2))
  (bind _spreadcurrent (Variables|/Game/UltimateFPSAnimationsKIT/Demo/PlayerMannequin/BP_PlayerCharacter.BP_PlayerCharacter_C|GetSpreadCurrent _asbp_player_character_2))
  (bind _playercamera (Variables|/Game/UltimateFPSAnimationsKIT/Demo/PlayerMannequin/BP_PlayerCharacter.BP_PlayerCharacter_C|GetPlayerCamera _asbp_player_character))
  (bind _returnvalue_4 (Transformation|GetWorldLocation _playercamera))
  (bind _returnvalue_5 (* _spreadcurrent 1e+04))
  (bind _returnvalue_6 (+ _bulletspread _returnvalue_5))
  (bind _returnvalue_7 (* _returnvalue_6 -1.0))
  (bind _outhit (Collision|LineTraceByChannel _returnvalue_4 (+ (+ (* (Math|Vector|GetForwardVector _playercamera) 2e+04) _returnvalue_4) (Math|Vector|MakeVector (Math|Random|RandomFloatinRange _returnvalue_7 _returnvalue_6) (Math|Random|RandomFloatinRange _returnvalue_7 _returnvalue_6) (Math|Random|RandomFloatinRange _returnvalue_7 _returnvalue_6))) "TraceTypeQuery1" false 0 "None")) ; CameraLineTrace
  (Collision|LineTraceByChannel _returnvalue_3 (.ImpactPoint (Collision|BreakHitResult _outhit)) "TraceTypeQuery1" false 0 "None" true "(R=0.000000,G=1.000000,B=0.110935,A=1.000000)") ; MuzzleLineTrace
  (return _returnvalue_3 (.ImpactPoint (Collision|BreakHitResult _outhit)) (Math|Rotator|FindLookatRotation (.TraceStart (Collision|BreakHitResult _outhit)) (.TraceEnd (Collision|BreakHitResult _outhit)))))

(fn SpawnBulletProjectile
  (params (MuzzleLocation :type Vector) (ImpactPoint :type Vector) (SpawnTransformLocation :type Vector) (ProjectileRotation :type Rotator))
  (Game|SpawnActorfromClass "/Game/UltimateFPSAnimationsKIT/Gun_Blueprints/BP_BulletDecal.BP_BulletDecal_C" (Math|Transform|MakeTransform SpawnTransformLocation (Math|Conversions|RotationFromXVector ImpactPoint) "0.020000,0.020000,0.020000") "Undefined" "OverrideRootScale" 0 0)
  (Game|SpawnActorfromClass "/Game/UltimateFPSAnimationsKIT/Gun_Blueprints/BP_Bullet.BP_Bullet_C" (Math|Transform|MakeTransform MuzzleLocation ProjectileRotation "0.080000,0.080000,0.080000") "Undefined" "OverrideRootScale" 0 0)
  (return))