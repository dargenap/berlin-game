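; M1911 pistol weapon Blueprint that handles hitscan firing and magazine ammo.
; Primary fire spends a round and line-traces forward from the skeletal mesh's Muzzle socket on the Visibility channel, applying point damage to the hit actor, with debug drawing and prints.
; BeginPlay fills the magazine and enables firing.
; A failed shot clears CanFire, and reload refills ammo without setting it back.
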(event Custom|eventPrimaryFire
  (bind _skeletalmesh (Variables|Default|GetSkeletalMesh))
  (bind _returnvalue (Transformation|GetSocketLocation _skeletalmesh "Muzzle"))
  (if (and (> (Variables|Default|GetcurrentAmmo) 0) (Variables|Default|GetcanFire))
    (Variables|Default|SetcanFire true)
    (Development|PrintString "shoot")
    (bind _output_get (Variables|Default|SetcurrentAmmo (- (Variables|Default|GetcurrentAmmo) 1)))
    (Development|PrintString (Utilities|String|ToString(Integer) _output_get))
    (bind (_outhit _returnvalue_2) (Collision|LineTraceByChannel _returnvalue (+ _returnvalue (* (Math|Vector|GetForwardVector (Transformation|GetSocketRotation _skeletalmesh "Muzzle")) 5e+03)) "TraceTypeQuery1" false 0 "ForDuration"))
    (if _returnvalue_2
      (Game|Damage|ApplyPointDamage (.HitActor (Collision|BreakHitResult _outhit)) 7e+01 (.Location (Collision|BreakHitResult _outhit)) _outhit))
    (else
      (Variables|Default|SetcanFire false))))

(event Custom|eventReload
  (Variables|Default|SetcurrentAmmo (Variables|Default|GetmagSize)))

(event EventBeginPlay
  (Variables|Default|SetcurrentAmmo (Variables|Default|GetmagSize))
  (Variables|Default|SetcanFire true))

(event Collision|EventActorBeginOverlap
  (params (OtherActor :type Actor%20Object%20Reference)))

(event EventTick
  (params (DeltaSeconds :type Float%20%28single-precision%29)))

(fn ConstructionScript)